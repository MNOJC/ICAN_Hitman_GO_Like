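; Lamp Blueprint that randomly flickers its point light together with the emissive material on its mesh.
; On BeginPlay it creates a dynamic lamp material, sets the default on/off state, then rolls against FlickeringChance to play a timeline driving IES brightness scale and emissive intensity.
; After a random delay, lamps on by default roll again, while off-by-default lamps are switched dark and stop cycling.
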(event `self.ReceiveBeginPlay`
  (bind _returnvalue (`PrimitiveComponent.CreateDynamicMaterialInstance` (`self.StaticMesh`) 1 "/Game/Assets/Material/M_Emissive_Lamps.M_Emissive_Lamps" "None"))
  (set `self.DynaicLampMaterial` _returnvalue)
  (if (`self.IsOnByDefault`)
    (`MaterialInstanceDynamic.SetScalarParameterValue` (`self.DynaicLampMaterial`) "EmissiveIntensity" (`LightComponent.IESBrightnessScale` (`self.PointLight`)))
    (else
      (`LightComponent.SetIESBrightnessScale` (`self.PointLight`) 0.0)
      (`MaterialInstanceDynamic.SetScalarParameterValue` (`self.DynaicLampMaterial`) "EmissiveIntensity" 0.0)))
  (if (> (`self.FlickeringChance`) (`KismetMathLibrary.RandomFloat`)) :!label _label
    (bind (_direction _lightflickering) (`Timeline|Timeline` :!via `PlayFromStart`)
      (:`Update`
        (`LightComponent.SetIESBrightnessScale` (`self.PointLight`) _lightflickering)
        (`MaterialInstanceDynamic.SetScalarParameterValue` (`self.DynaicLampMaterial`) "EmissiveIntensity" _lightflickering))
      (:`Finished`
        (`KismetSystemLibrary.Delay` (`KismetMathLibrary.RandomFloatInRange` (`self.MinimumDelayBetweenFlickers`) (`self.MaximumDelayBetweenFlicker`)) :!label _label_2)
        (if (`self.IsOnByDefault`)
          (`MaterialInstanceDynamic.SetScalarParameterValue` (`self.DynaicLampMaterial`) "EmissiveIntensity" (`LightComponent.IESBrightnessScale` (`self.PointLight`)))
          (goto _label)
          (else
            (`LightComponent.SetIESBrightnessScale` (`self.PointLight`) 0.0)
            (`MaterialInstanceDynamic.SetScalarParameterValue` (`self.DynaicLampMaterial`) "EmissiveIntensity" 0.0)))))
    (else
      (goto _label_2))))

(fn `UserConstructionScript`)