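; Flickering lamp actor that animates a spotlight and the emissive material on its lamp mesh together.
; BeginPlay creates a dynamic emissive material and sets the on/off state, then a random chance roll plays a timeline driving IES brightness and emissive intensity.
; After a random delay, lamps on by default match emissive to the spotlight and roll again, while off-by-default lamps go dark and stop after that single cycle.
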(event `self.ReceiveBeginPlay`
  (bind _spotlight (`self.SpotLight`))
  (bind _returnvalue (`PrimitiveComponent.CreateDynamicMaterialInstance` (`self.SM_lampe01`) 1 "/Game/Assets/Material/M_Emissive_Lamps.M_Emissive_Lamps" "None"))
  (set `self.DynaicLampMaterial` _returnvalue)
  (if (`self.IsOnByDefault`)
    (`MaterialInstanceDynamic.SetScalarParameterValue` (`self.DynaicLampMaterial`) "EmissiveIntensity" (`LightComponent.IESBrightnessScale` _spotlight))
    (else
      (`LightComponent.SetIESBrightnessScale` _spotlight 0.0)
      (`MaterialInstanceDynamic.SetScalarParameterValue` (`self.DynaicLampMaterial`) "EmissiveIntensity" 0.0)))
  (if (> (`self.FlickeringChance`) (`KismetMathLibrary.RandomFloat`)) :!label _label
    (bind (_direction _lightflickering) (`Timeline|Timeline` :!via `PlayFromStart`)
      (:`Update`
        (`LightComponent.SetIESBrightnessScale` (`self.SpotLight`) _lightflickering)
        (`MaterialInstanceDynamic.SetScalarParameterValue` (`self.DynaicLampMaterial`) "EmissiveIntensity" _lightflickering))
      (:`Finished`
        (`KismetSystemLibrary.Delay` (`KismetMathLibrary.RandomFloatInRange` (`self.MinimumDelayBetweenFlickers`) (`self.MaximumDelayBetweenFlicker`)) :!label _label_2)
        (if (`self.IsOnByDefault`)
          (`MaterialInstanceDynamic.SetScalarParameterValue` (`self.DynaicLampMaterial`) "EmissiveIntensity" (`LightComponent.IESBrightnessScale` (`self.SpotLight`)))
          (goto _label)
          (else
            (`LightComponent.SetIESBrightnessScale` (`self.SpotLight`) 0.0)
            (`MaterialInstanceDynamic.SetScalarParameterValue` (`self.DynaicLampMaterial`) "EmissiveIntensity" 0.0)))))
    (else
      (goto _label_2))))

(fn `UserConstructionScript`)