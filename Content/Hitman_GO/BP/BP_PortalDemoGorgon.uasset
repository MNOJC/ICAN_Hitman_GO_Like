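; Portal actor for the Hitman GO project that animates its cover open and closed in response to enemy pawn portal events.
; On BeginPlay it creates a dynamic cover material, then after a short delay binds to the first found BP_HGOEnemyPawn's portal created and crossed events.
; When the event's node matches NodeID, opposing timelines drive the material's opening parameter, each stopping the other.
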(event `OpenPortal`
  (`|ExecutionSequence`
    (:`then_0`
      (bind (_direction _closing) (`Timeline|CloseTimeline` :!via `Stop` :!label _label)
        (:`Update`
          (`MaterialInstanceDynamic.SetScalarParameterValue` (`self.PortalCoverDynamicMaterial`) (`self.OpeningParameterName`) _closing))))
    (:`then_1`
      (bind (_direction_2 _opening) (`Timeline|OpenTimeline` :!via `PlayFromStart` :!label _label_2)
        (:`Update`
          (`MaterialInstanceDynamic.SetScalarParameterValue` (`self.PortalCoverDynamicMaterial`) (`self.OpeningParameterName`) _opening))))))

(event `ClosePortal`
  (`|ExecutionSequence`
    (:`then_0`
      (goto _label_2 :!via `Stop`))
    (:`then_1`
      (goto _label :!via `PlayFromStart`))))

(event `self.ReceiveBeginPlay`
  (bind _returnvalue (`PrimitiveComponent.CreateDynamicMaterialInstance` (`self.PortalMesh`) 1 "/Game/Hitman_GO/Art/Materials/Instances/MI_PortalCover.MI_PortalCover" "None"))
  (bind _output_get (set `self.PortalCoverDynamicMaterial` _returnvalue))
  (`MaterialInstanceDynamic.SetScalarParameterValue` _output_get (`self.OpeningParameterName`) 0.0)
  (`KismetSystemLibrary.Delay` 0.2)
  (bind _returnvalue_2 (`GameplayStatics.GetActorOfClass` "/Game/Hitman_GO/Core/BP_HGOEnemyPawn.BP_HGOEnemyPawn_C"))
  (add `HGOEnemyPawn.OnPortalCreated` _returnvalue_2 (delegate `OnPortalCreated_Event`))
  (add `HGOEnemyPawn.OnPortalCrossed` _returnvalue_2 (delegate `OnPortalCrossed_Event`)))

(event `OnPortalCreated_Event`
  (params (PortalNodeID :type Integer))
  (if (`KismetArrayLibrary.Array_Contains` (`self.NodeID`) PortalNodeID)
    (`self.OpenPortal`)))

(event `OnPortalCrossed_Event`
  (params (PortalNodeID :type Integer))
  (if (`KismetArrayLibrary.Array_Contains` (`self.NodeID`) PortalNodeID)
    (`self.ClosePortal`)))

(fn `UserConstructionScript`)