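; BP_FlickeringLamp is a lamp actor that flickers at random intervals, driving a RectLight and its mesh's emissive material together.
; InitLamp creates the dynamic material, picks the normal or upside-down light color, and starts flickering if the lamp is on by default.
; StartFlickering loops a random chance roll, a timeline that scales IES brightness and emissive intensity, and a random delay.
; StopFlickering stops the timeline and darkens both.
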(event `StartFlickering`
  (if (not (`self.IsFlickering`))
    (set `self.IsFlickering` true)
    (`MaterialInstanceDynamic.SetScalarParameterValue` (`self.DynamicLampMaterial`) "EmissiveIntensity" (`self.MaximumEmissiveIntensity`))
    (if (> (`self.FlickeringChance`) (`KismetMathLibrary.RandomFloat`)) :!label _label
      (bind (_direction _lightflickering) (`Timeline|Timeline_0` :!via `PlayFromStart` :!label _label_2)
        (:`Update`
          (`LightComponent.SetIESBrightnessScale` (`self.RectLight`) (* _lightflickering (`self.MaximumLightIntensity`)))
          (`MaterialInstanceDynamic.SetScalarParameterValue` (`self.DynamicLampMaterial`) "EmissiveIntensity" (* _lightflickering (`self.MaximumEmissiveIntensity`))))
        (:`Finished`
          (`KismetSystemLibrary.Delay` (`KismetMathLibrary.RandomFloatInRange` (`self.MinimumDelayBetweenFlickers`) (`self.MaximumDelayBetweenFlicker`)) :!label _label_3)
          (if (`self.IsFlickering`)
            (`MaterialInstanceDynamic.SetScalarParameterValue` (`self.DynamicLampMaterial`) "EmissiveIntensity" (`self.MaximumEmissiveIntensity`))
            (`LightComponent.SetIESBrightnessScale` (`self.RectLight`) (`self.MaximumLightIntensity`))
            (goto _label)
            (else
              (`LightComponent.SetIESBrightnessScale` (`self.RectLight`) 0.0)
              (`MaterialInstanceDynamic.SetScalarParameterValue` (`self.DynamicLampMaterial`) "EmissiveIntensity" 0.0)))))
      (else
        (goto _label_3)))))

(event `StopFlickering`
  (if (`self.IsFlickering`)
    (`LightComponent.SetIESBrightnessScale` (`self.RectLight`) 0.0)
    (`MaterialInstanceDynamic.SetScalarParameterValue` (`self.DynamicLampMaterial`) "EmissiveIntensity" 0.0)
    (set `self.IsFlickering` false)
    (goto _label_2 :!via `Stop`)))

(event `self.ReceiveBeginPlay`)

(event `InitLamp`
  (params (NormalColor :type "LinearColor Structure") (UpsidedownColor :type "LinearColor Structure") (IsUpsideDown :type Boolean))
  (bind _returnvalue (`PrimitiveComponent.CreateDynamicMaterialInstance` (`self.SM_Lamp`) (`self.EmissiveMaterialIndex`) (`self.EmissiveMaterial`) "None"))
  (set `self.DynamicLampMaterial` _returnvalue)
  (set `self.FinalColor` (`KismetMathLibrary.SelectColor` UpsidedownColor NormalColor IsUpsideDown))
  (`LightComponent.SetLightColor` (`self.RectLight`) (`self.FinalColor`) true)
  (if (`self.IsOnByDefault`)
    (`MaterialInstanceDynamic.SetScalarParameterValue` (`self.DynamicLampMaterial`) "EmissiveIntensity" (`self.MaximumEmissiveIntensity`))
    (`LightComponent.SetIESBrightnessScale` (`self.RectLight`) (`self.MaximumLightIntensity`))
    (`self.StartFlickering`)
    (else
      (`LightComponent.SetIESBrightnessScale` (`self.RectLight`) 0.0)
      (`MaterialInstanceDynamic.SetScalarParameterValue` (`self.DynamicLampMaterial`) "EmissiveIntensity" 0.0))))

(fn `UpdateColor`
  (`LightComponent.SetLightColor` (`self.RectLight`) (`self.FinalColor`) true))

(fn `UserConstructionScript`
  (`LightComponent.SetLightColor` (`self.RectLight`) (`self.FinalColor`) true))