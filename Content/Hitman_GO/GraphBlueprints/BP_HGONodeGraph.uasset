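; Node marker for the Hitman GO graph board, displayed as a small scaled-down plane.
; On BeginPlay it sets the plane mesh and picks a red or yellow decal material based on whether the node is upside down.
; After a brief delay it creates a dynamic material instance and tints its Color parameter by node type, distinguishing normal, start, goal, blocked and player or enemy portal nodes.
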(event `self.ReceiveBeginPlay`
  (bind (_nodeid _position _nodetype _bisupsidedownnode) (break `NodeData` (`self.NodeData`)))
  (`self.SetStaticMesh` self "/Engine/BasicShapes/Plane.Plane")
  (`self.SetWorldScale3D` self (0.05 0.05 0.05))
  (`self.SetMaterial` self 0 (select `bool` _bisupsidedownnode :`false` "/Game/Hitman_GO/Art/Materials/Instances/MI_DecalNodeYellow.MI_DecalNodeYellow" :`true` "/Game/Hitman_GO/Art/Materials/Instances/MI_DecalNodeRed.MI_DecalNodeRed" :!type "MaterialInterface Object Reference"))
  (`KismetSystemLibrary.Delay` 0.1)
  (bind _returnvalue (`self.CreateDynamicMaterialInstance` self 0 null "None"))
  (`MaterialInstanceDynamic.SetVectorParameterValue` _returnvalue "Color" (select `ENodeType` _nodetype :`Normal` (struct :`R` 0.270498 :`G` 0.973445 :`B` 1.0 :`A` 1.0) :`Start` (struct :`R` 0.093059 :`G` 1.0 :`A` 1.0) :`Goal` (struct :`R` 1.0 :`G` 0.019382 :`A` 1.0) :`Blocked` (struct :`R` 0.973445 :`G` 1.0 :`B` 0.48515 :`A` 1.0) :`PlayerPortal` (struct :`R` 0.313989 :`G` 0.181164 :`B` 1.0 :`A` 1.0) :`EnemyPortal` (struct :`G` 0.013702 :`B` 1.0 :`A` 1.0) :!type "LinearColor Structure")))

(fn `UserConstructionScript`)