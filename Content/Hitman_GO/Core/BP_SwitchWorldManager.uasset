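; Manages the Hitman GO board's switch between normal and upside-down worlds, triggered by a game mode event.
; Tick sinks "Root"-tagged meshes with randomized delays and speeds, then unloads the old streamed level.
; A timeline flips the board and moves the camera, then loads the new level, raises its meshes, notifies the level generator and animates the pawn in.
; With animation disabled, it only runs those last two steps after a delay.
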(event `self.ReceiveTick`
  (params (DeltaSeconds :type "Float (single-precision)"))
  (bind _managedmeshes (`self.ManagedMeshes`))
  (if (`self.RunTransition`)
    (set `self.Time` (+ (`self.Time`) DeltaSeconds))
    (for (_array_element _array_index) _managedmeshes
      (bind (_meshactor _delaystarting _elapsedtime _zoffset _speed _rotation _startingloc) (break `/Game/Hitman_GO/Structures/S_BoardAnim` _array_element))
      (if (>= (`self.Time`) _delaystarting)
        (bind _returnvalue (`self.K2_GetActorLocation` _meshactor))
        (bind _returnvalue_2 (select `bool` (`self.InDown`) :`false` (`KismetMathLibrary.MakeVector` (.x _startingloc) (.y _startingloc) (+ (.z _startingloc) 0.0)) :`true` (`KismetMathLibrary.MakeVector` (.x _startingloc) (.y _startingloc) (- (.z _startingloc) _zoffset))))
        (`self.K2_SetActorLocation` _meshactor (`KismetMathLibrary.VInterpTo_Constant` _returnvalue _returnvalue_2 (`GameplayStatics.GetWorldDeltaSeconds`) _speed) false false)
        (if (`KismetMathLibrary.NearlyEqual_FloatFloat` (`KismetMathLibrary.Vector_Distance` _returnvalue _returnvalue_2) 0.0 0.1)
          (bind (_meshactor_2 _delaystarting_2 _elapsedtime_2 _zoffset_2 _speed_2 _rotation_2 _startingloc_2) (break `/Game/Hitman_GO/Structures/S_BoardAnim` _array_element))
          (`|VariableSetRef` (`|GetArrayItem` _managedmeshes _array_index) (make `/Game/Hitman_GO/Structures/S_BoardAnim` _meshactor_2 _delaystarting_2 _elapsedtime_2 _zoffset_2 _speed_2 _rotation_2 _startingloc_2 true))
          (if (`self.isBoardAnimCompleted`)
            (set `self.RunTransition` false)
            (if (`self.InDown`)
              (`GameplayStatics.UnloadStreamLevelBySoftObjectPtr` (`self.LevelToUnload`))
              (`LightComponent.SetIntensity` (`SpotLight.SpotLightComponent` (`self.SpotLightRef`)) 8.0)
              (`self.PlayBoardAnim`))))))))

(event `self.ReceiveBeginPlay`
  (bind _output_get (set `self.LevelToLoad` (`self.LevelNormal`)))
  (`GameplayStatics.LoadStreamLevelBySoftObjectPtr` _output_get true)
  (`self.UnhideMeshActors`)
  (bind _asbp_hgogame_mode (cast `/Game/Hitman_GO/Core/BP_HGOGameMode` (`GameplayStatics.GetGameMode`)))
  (add `HGOGameMode.OnSwitchWorldGraph` _asbp_hgogame_mode (delegate `OnSwitchWorldGraph_Event`)))

(event `OnSwitchWorldGraph_Event`
  (params (bToUpsidedown :type Boolean))
  (`self.SwitchWorld` bToUpsidedown))

(event `PlayBoardAnim`
  (bind _defaultboardtransform_location (`KismetMathLibrary.BreakTransform` (`self.DefaultBoardTransform`)))
  (bind _camera (`self.Camera`))
  (bind _returnvalue (`GameplayStatics.GetActorOfClass` "/Game/Hitman_GO/Camera/BP_HGOCamera.BP_HGOCamera_C"))
  (set `self.Camera` _returnvalue)
  (set `self.DefaultBoardTransform` (`self.GetTransform` (`self.BoardRef`)))
  (bind (_direction _rotationalpha _movement _scalealpha _valuealphacam) (`Timeline|BoardAnim` :!via `PlayFromStart`)
    (:`Update`
      (`self.K2_SetActorRotation` (`self.BoardRef`) (`KismetMathLibrary.RLerp` (struct) (struct :`Pitch` 180.0) _rotationalpha) false)
      (bind (_returnvalue_x _returnvalue_y _returnvalue_z) (`KismetMathLibrary.BreakVector` (+ _defaultboardtransform_location _movement)))
      (`self.K2_SetActorLocation` (`self.BoardRef`) (`KismetMathLibrary.MakeVector` _returnvalue_x _returnvalue_y _returnvalue_z) false false)
      (set `SpringArmComponent.TargetArmLength` (`KismetMathLibrary.Lerp` 160.0 220.0 _valuealphacam) (`HGOCamera.SpringArm` _camera))
      (`CameraComponent.SetFieldOfView` (`HGOCamera.Camera` _camera) (`KismetMathLibrary.Lerp` 60.0 70.0 _valuealphacam)))
    (:`Finished`
      (bind _returnvalue_2 (`GameplayStatics.GetActorOfClass` "/Game/Hitman_GO/GraphBlueprints/BP_HGOTacticalLevelGenerator.BP_HGOTacticalLevelGenerator_C"))
      (`HGOTacticalLevelGenerator.OnBoardFlipAnimCompleted` _returnvalue_2)
      (`GameplayStatics.LoadStreamLevelBySoftObjectPtr` (`self.LevelToLoad`) true)
      (`LightComponent.SetIntensity` (`SpotLight.SpotLightComponent` (`self.SpotLightRef`)) 0.0)
      (`self.StartUpsideDownSpawn`)
      (bind _returnvalue_3 (`GameplayStatics.GetActorOfClass` "/Game/Hitman_GO/Core/BP_HGOPlayerPawn.BP_HGOPlayerPawn_C"))
      (bind (_returnvalue_location _returnvalue_rotation) (`KismetMathLibrary.BreakTransform` (`self.GetTransform` _returnvalue_3)))
      (`/Game/Hitman_GO/Core/AC_PawnAnimation.PlayAnimationBoardIn` (`/Game/Hitman_GO/Core/BP_HGOPlayerPawn.AC_PawnAnimation` _returnvalue_3) (`KismetMathLibrary.MakeTransform` _returnvalue_location _returnvalue_rotation)))))

(event `SwitchWorld`
  (params (ToUpsideDown :type Boolean))
  (bind _output_get (set `self.To Upside Down` ToUpsideDown))
  (set `self.InDown` true)
  (if _output_get
    (`FMODBlueprintStatics.PlayEvent2D` "/Game/FMOD/Events/Player/SD_PlayerBackToUpside.SD_PlayerBackToUpside")
    (set `self.LevelToLoad` (`self.LevelUpsideDown`))
    (set `self.LevelToUnload` (`self.LevelNormal`))
    (else
      (`FMODBlueprintStatics.PlayEvent2D` "/Game/FMOD/Events/Player/SD_PlayerBackToRightSide.SD_PlayerBackToRightSide")
      (set `self.LevelToLoad` (`self.LevelNormal`))
      (set `self.LevelToUnload` (`self.LevelUpsideDown`))))
  (`self.SetManagedMeshes` :!label _label)
  (set `self.Time` 0.0)
  (if (`self.InDown`)
    (if (`self.PlayAnimation`)
      (set `self.RunTransition` true)
      (else
        (`self.SkipAnimation`)))
    (else
      (for _array_element (`self.ManagedMeshes`)
        (bind (_meshactor _delaystarting _elapsedtime _zoffset _speed _rotation _startingloc) (break `/Game/Hitman_GO/Structures/S_BoardAnim` _array_element))
        (`self.K2_SetActorLocation` _meshactor (`KismetMathLibrary.MakeVector` (.x _startingloc) (.y _startingloc) (- (.z _startingloc) _zoffset)) false false)
        (`self.SetActorHiddenInGame` _meshactor false))
      (`GameplayStatics.LoadStreamLevelBySoftObjectPtr` (`self.LevelToLoad`) true)
      (set `self.RunTransition` true))))

(event `StartUpsideDownSpawn`
  (set `self.InDown` false)
  (goto _label))

(event `SkipAnimation`
  (`KismetSystemLibrary.Delay` 4.5)
  (bind _returnvalue (`GameplayStatics.GetActorOfClass` "/Game/Hitman_GO/GraphBlueprints/BP_HGOTacticalLevelGenerator.BP_HGOTacticalLevelGenerator_C"))
  (`HGOTacticalLevelGenerator.OnBoardFlipAnimCompleted` _returnvalue)
  (bind _returnvalue_2 (`GameplayStatics.GetActorOfClass` "/Game/Hitman_GO/Core/BP_HGOPlayerPawn.BP_HGOPlayerPawn_C"))
  (bind (_returnvalue_location _returnvalue_rotation) (`KismetMathLibrary.BreakTransform` (`self.GetTransform` _returnvalue_2)))
  (`/Game/Hitman_GO/Core/AC_PawnAnimation.PlayAnimationBoardIn` (`/Game/Hitman_GO/Core/BP_HGOPlayerPawn.AC_PawnAnimation` _returnvalue_2) (`KismetMathLibrary.MakeTransform` _returnvalue_location _returnvalue_rotation)))

(fn `isBoardAnimCompleted`
  (returns (Completed :type Boolean))
  (for _array_element (`self.ManagedMeshes`)
    (if (not (`.Finished_11_2C1DAB80487EA1122E3C209221745DAD` (break `/Game/Hitman_GO/Structures/S_BoardAnim` _array_element)))
      (return false)))
  (return true))

(fn `SetManagedMeshes`
  (`KismetArrayLibrary.Array_Clear` (`self.ManagedMeshes`))
  (bind _outactors (`GameplayStatics.GetAllActorsWithTag` "Root"))
  (for _array_element _outactors
    (bind _returnvalue (* (.z (`.BoxExtent` (`self.GetActorBounds` _array_element false false))) 3.0))
    (`KismetArrayLibrary.Array_Add` (`self.ManagedMeshes`) (make `/Game/Hitman_GO/Structures/S_BoardAnim` _array_element (`KismetMathLibrary.RandomFloatInRange` 0.0 1.0) 0.0 (`KismetMathLibrary.SelectFloat` 20.0 _returnvalue (< _returnvalue 20.0)) (`KismetMathLibrary.RandomFloatInRange` 35.0 45.0) (struct) (`self.K2_GetActorLocation` _array_element))))
  (return))

(fn `UnhideMeshActors`
  (bind _outactors (`GameplayStatics.GetAllActorsWithTag` "Root"))
  (for _array_element _outactors
    (`self.SetActorHiddenInGame` _array_element false)))

(fn `UserConstructionScript`)