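; Enemy detection indicator for the Hitman GO game that lights its SMLight mesh yellow when an enemy pawn stands on one of its DetectedNodeIDs, and black otherwise.
; After a short BeginPlay delay, it finds all BP_HGOEnemyPawn actors, binds to each GraphMovementComponent's movement-completed event and sets the initial color.
; Each check creates a dynamic material instance and reflects only the enemy just evaluated, so the last one wins.
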(event `self.ReceiveBeginPlay`
  (`KismetSystemLibrary.Delay` 0.2)
  (bind _outactors (`GameplayStatics.GetAllActorsOfClass` "/Game/Hitman_GO/Core/BP_HGOEnemyPawn.BP_HGOEnemyPawn_C"))
  (for _array_element _outactors
    (bind _graphmovementcomponent (`HGOEnemyPawn.GraphMovementComponent` _array_element))
    (add `HGOGraphMovementComponent.OnMovementCompleted` _graphmovementcomponent (delegate `OnMovementCompleted_Event`))
    (if (`KismetArrayLibrary.Array_Contains` (`self.DetectedNodeIDs`) (`.NodeID` (break `NodeData` (`HGONodeGraphComponent.NodeData` (`HGOGraphMovementComponent.GetCurrentNode` _graphmovementcomponent)))))
      (bind _returnvalue (`PrimitiveComponent.CreateDynamicMaterialInstance` (`self.SM_Light`) 0 null "None"))
      (`MaterialInstanceDynamic.SetVectorParameterValue` _returnvalue "Color" (struct :`R` 0.723055 :`G` 0.637597 :`A` 1.0))
      (else
        (bind _returnvalue_2 (`PrimitiveComponent.CreateDynamicMaterialInstance` (`self.SM_Light`) 0 null "None"))
        (`MaterialInstanceDynamic.SetVectorParameterValue` :`self` _returnvalue_2 :`ParameterName` "Color")))))

(event `OnMovementCompleted_Event`
  (params (NewNode :type Integer))
  (bind _sm_light (`self.SM_Light`))
  (if (`KismetArrayLibrary.Array_Contains` (`self.DetectedNodeIDs`) NewNode)
    (bind _returnvalue (`PrimitiveComponent.CreateDynamicMaterialInstance` _sm_light 0 null "None"))
    (`MaterialInstanceDynamic.SetVectorParameterValue` _returnvalue "Color" (struct :`R` 1.0 :`G` 0.878443 :`A` 1.0))
    (else
      (bind _returnvalue_2 (`PrimitiveComponent.CreateDynamicMaterialInstance` _sm_light 0 null "None"))
      (`MaterialInstanceDynamic.SetVectorParameterValue` _returnvalue_2 "Color" (struct :`A` 1.0)))))

(fn `UserConstructionScript`)