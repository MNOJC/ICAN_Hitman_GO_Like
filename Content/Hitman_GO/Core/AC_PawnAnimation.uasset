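; Actor component for Hitman GO pawns that animates its owner leaving and entering the board.
; Board-out sinks the owner 10 units while shrinking it toward zero scale, and death reuses this animation.
; Board-in places it 10 units below a given transform, then eases it toward world Z zero.
; Both use looping per-frame timers with VInterpTo, cleared once the location is within one unit of target.
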(event `TriggerBoardOutAnim`
  (set `self.DefaultTransform` (`Actor.GetTransform` (`self.GetOwner`)))
  (bind _returnvalue (`KismetSystemLibrary.K2_SetTimerDelegate` (delegate `BoardOutAnimTick`) 0.0001 true true))
  (set `self.BoardOutHandle` _returnvalue))

(event `BoardOutAnimTick`
  (bind _returnvalue (`self.GetOwner`))
  (bind _defaulttransform_location (`KismetMathLibrary.BreakTransform` (`self.DefaultTransform`)))
  (bind _returnvalue_2 (`Actor.K2_GetActorLocation` _returnvalue))
  (bind _returnvalue_3 (+ _defaulttransform_location (0.0 0.0 -10.0)))
  (`Actor.K2_SetActorLocation` _returnvalue (`KismetMathLibrary.VInterpTo` _returnvalue_2 _returnvalue_3 (`GameplayStatics.GetWorldDeltaSeconds`) 1.0) false false)
  (`Actor.SetActorScale3D` (`self.GetOwner`) (`KismetMathLibrary.VInterpTo` (`Actor.GetActorScale3D` (`self.GetOwner`)) (0.0 0.0 0.0) (`GameplayStatics.GetWorldDeltaSeconds`) 2.0))
  (if (< (`KismetMathLibrary.Vector_Distance` _returnvalue_2 _returnvalue_3) 1.0)
    (`KismetSystemLibrary.K2_ClearAndInvalidateTimerHandle` (`self.BoardOutHandle`))))

(event `TriggerBoardInAnim`
  (params (DefaultTransform :type "Transform Structure"))
  (`Actor.K2_SetActorTransform` (`self.GetOwner`) (`KismetMathLibrary.MakeTransform` (`KismetMathLibrary.MakeVector` (.x (.location DefaultTransform)) (.y (.location DefaultTransform)) (+ (.z (.location DefaultTransform)) -10.0)) (.rotation DefaultTransform) (.scale DefaultTransform)) false false)
  (set `self.DefaultTransform` DefaultTransform)
  (bind _returnvalue (`KismetSystemLibrary.K2_SetTimerDelegate` (delegate `BoardInAnmTick`) 0.0001 true true))
  (set `self.BoardInHandle` _returnvalue))

(event `BoardInAnmTick`
  (bind _returnvalue (`self.GetOwner`))
  (bind _defaulttransform_location (`KismetMathLibrary.BreakTransform` (`self.DefaultTransform`)))
  (bind (_defaulttransform_location_2 _defaulttransform_rotation _defaulttransform_scale) (`KismetMathLibrary.BreakTransform` (`self.DefaultTransform`)))
  (bind _returnvalue_2 (`Actor.K2_GetActorLocation` _returnvalue))
  (bind _returnvalue_3 (`KismetMathLibrary.MakeVector` (.x _defaulttransform_location) (.y _defaulttransform_location)))
  (`KismetSystemLibrary.PrintString` (`KismetStringLibrary.Conv_VectorToString` _returnvalue_2))
  (`Actor.K2_SetActorLocation` _returnvalue (`KismetMathLibrary.VInterpTo` _returnvalue_2 _returnvalue_3 (`GameplayStatics.GetWorldDeltaSeconds`) 2.5) false false)
  (`Actor.SetActorScale3D` (`self.GetOwner`) (`KismetMathLibrary.VInterpTo` (`Actor.GetActorScale3D` (`self.GetOwner`)) _defaulttransform_scale (`GameplayStatics.GetWorldDeltaSeconds`) 2.0))
  (if (< (`KismetMathLibrary.Vector_Distance` _returnvalue_2 _returnvalue_3) 1.0)
    (`KismetSystemLibrary.K2_ClearAndInvalidateTimerHandle` (`self.BoardInHandle`))))

(fn `InitPawn`)

(fn `PlayAnimationBoardIn`
  (params (DefaultTransform :type "Transform Structure"))
  (`self.TriggerBoardInAnim` DefaultTransform))

(fn `PlayAnimationBoardOut`
  (`self.TriggerBoardOutAnim`))

(fn `PlayDeathFromOtherWorld`
  (`self.PlayAnimationBoardOut`))