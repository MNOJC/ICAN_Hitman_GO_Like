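; Enemy pawn for the Hitman GO-style board game, handling hover highlighting and visibility across the normal and upside-down worlds.
; Cursor hover on the enemy mesh swaps in a dynamic overlay material with a thicker outline, thinned again when hover ends.
; Passing through a portal combines the parent's result with the player's current world to show or hide the mesh.
; The game mode's world-switch event is bound on BeginPlay, but its handler is empty.
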(event `self.ReceiveBeginPlay`
  (`parent.ReceiveBeginPlay`)
  (bind _asbp_hgogame_mode (cast `/Game/Hitman_GO/Core/BP_HGOGameMode` (`GameplayStatics.GetGameMode`)))
  (bind _output_get (set `self.HGOGameMode` _asbp_hgogame_mode))
  (add `HGOGameMode.OnSwitchWorldGraph` _output_get (delegate `OnSwitchWorldGraph_Event`)))

(event `OnSwitchWorldGraph_Event`
  (params (bToUpsidedown :type Boolean)))

(event `self.EnemyMeshComponent.OnBeginCursorOver`
  (params (TouchedComponent :type "PrimitiveComponent Object Reference"))
  (bind _overlaymaterial (`self.OverlayMaterial`))
  (bind _returnvalue (`PrimitiveComponent.CreateDynamicMaterialInstance` _overlaymaterial 0 (`MeshComponent.GetOverlayMaterial` _overlaymaterial) "None"))
  (`MaterialInstanceDynamic.SetScalarParameterValue` _returnvalue "Thickness" 0.4)
  (`MeshComponent.SetOverlayMaterial` (`self.EnemyMeshComponent`) _returnvalue))

(event `self.EnemyMeshComponent.OnEndCursorOver`
  (params (TouchedComponent :type "PrimitiveComponent Object Reference"))
  (bind _overlaymaterial (`self.OverlayMaterial`))
  (bind _returnvalue (`PrimitiveComponent.CreateDynamicMaterialInstance` _overlaymaterial 0 (`MeshComponent.GetOverlayMaterial` _overlaymaterial) "None"))
  (`MaterialInstanceDynamic.SetScalarParameterValue` _returnvalue "Thickness" 0.2)
  (`MeshComponent.SetOverlayMaterial` (`self.EnemyMeshComponent`) _returnvalue))

(fn `OnEnemyPassThroughPortal`
  (returns (ReturnValue :type Boolean))
  (bind _returnvalue (`parent.OnEnemyPassThroughPortal`))
  (bind _returnvalue_2 (`GameplayStatics.GetActorOfClass` "/Game/Hitman_GO/Core/BP_HGOPlayerPawn.BP_HGOPlayerPawn_C"))
  (if _returnvalue
    (bind _binupsidedownworld (`HGOGraphMovementComponent.bInUpsideDownWorld` (`HGOPlayerPawn.GraphMovementComponent` _returnvalue_2)))
    (`SceneComponent.SetVisibility` (`self.EnemyMeshComponent`) (select `bool` _binupsidedownworld :`true` true) false)
    (else
      (`SceneComponent.SetVisibility` (`self.EnemyMeshComponent`) (select `bool` _binupsidedownworld :`false` true) false)))
  (return _returnvalue))

(fn `UserConstructionScript`)