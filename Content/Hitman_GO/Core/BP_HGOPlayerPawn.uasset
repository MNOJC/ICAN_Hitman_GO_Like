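; Player pawn for a Hitman GO-style turn-based game that turns gameplay events into animation and UI feedback.
; On BeginPlay it caches game mode and HUD, then binds death, level completion, world switch, turn and input-block events.
; Handlers play animations, show the death screen, update ability HUD, load the main map, or show an input indicator during unblocked player turns.
; The swipe overlap handler only casts to enemy pawn.
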(event `self.ReceiveBeginPlay`
  (add `self.OnPlayerDeath` (delegate `OnPlayerDeath_Event`))
  (add `self.OnLevelComplete` (delegate `OnLevelComplete_Event`))
  (add `self.OnAbilityCooldownUpdated` (delegate `OnAbilityCooldownUpdated_Event`))
  (bind _asbp_hgogame_mode (cast `/Game/Hitman_GO/Core/BP_HGOGameMode` (`GameplayStatics.GetGameMode`)))
  (set `self.HGOGameMode` _asbp_hgogame_mode)
  (bind _asbp_main_hud (cast `/Game/Hitman_GO/UI/BP_MainHUD` (`PlayerController.GetHUD` (`GameplayStatics.GetPlayerController` 0))))
  (set `self.HGOMainHUD` _asbp_main_hud)
  (add `HGOGameMode.OnSwitchWorldGraph` (`self.HGOGameMode`) (delegate `OnSwitchWorldGraph_Event`))
  (add `self.OnInputBlocked` (delegate `OnInputBlocked_Event`))
  (add `HGOTacticalTurnManager.OnTurnChanged` (subsystem `HGOTacticalTurnManager`) (delegate `OnTurnChanged_Event`)))

(event `OnPlayerDeath_Event` :!signature `self.OnPlayerDeath`
  (params (bKillInOtherWorld :type Boolean))
  (`KismetSystemLibrary.Delay` 1.0)
  (`/Game/Hitman_GO/Core/AC_PawnAnimation.PlayDeathFromOtherWorld` (`self.AC_PawnAnimation`))
  (`KismetSystemLibrary.Delay` 0.2)
  (bind _returnvalue (`|CreateWidget` "/Game/Hitman_GO/UI/WBP_DeathScreen.WBP_DeathScreen_C"))
  (`UserWidget.AddToViewport` _returnvalue 0))

(event `OnAbilityCooldownUpdated_Event` :!signature `self.OnAbilityCooldownUpdated`
  (params (NewCooldown :type Integer))
  (`/Game/Hitman_GO/UI/W_PlayerInterface.UpdateAbilityCooldown` (`/Game/Hitman_GO/UI/BP_MainHUD.PlayerInterface` (`self.HGOMainHUD`)) NewCooldown))

(event `OnLevelComplete_Event`
  (`GameplayStatics.OpenLevelBySoftObjectPtr` "/Game/Hitman_GO/Levels/L_MainMap.L_MainMap"))

(event `OnSwitchWorldGraph_Event`
  (params (bToUpsidedown :type Boolean))
  (`/Game/Hitman_GO/Core/AC_PawnAnimation.PlayAnimationBoardOut` (`self.AC_PawnAnimation`)))

(event `OnInputBlocked_Event` :!signature `self.OnInputBlocked`
  (params (bIsBlocked :type Boolean))
  (set `self.InputBlocked` bIsBlocked)
  (`self.updateInputFeedback`))

(event `OnTurnChanged_Event`
  (params (NewTurnState :type "ETurnState Enum" :default "PlayerTurn"))
  (set `self.Turn State` NewTurnState)
  (`self.updateInputFeedback`))

(event `self.CollisionSwipeComponent.OnComponentBeginOverlap`
  (params (OverlappedComponent :type "PrimitiveComponent Object Reference") (OtherActor :type "Actor Object Reference") (OtherComp :type "PrimitiveComponent Object Reference") (OtherBodyIndex :type Integer) (bFromSweep :type Boolean) (SweepResult :type "HitResult Structure (by ref)"))
  (cast `/Game/Hitman_GO/Core/BP_HGOEnemyPawn` OtherActor))

(event `self.OnAbilityBecameAvailable`
  (`/Game/Hitman_GO/UI/W_PlayerInterface.UpdateAbilityAvailability` (`/Game/Hitman_GO/UI/BP_MainHUD.PlayerInterface` (`self.HGOMainHUD`)) true))

(event `self.OnAbilityBecameUnavailable`
  (`/Game/Hitman_GO/UI/W_PlayerInterface.UpdateAbilityAvailability` (`/Game/Hitman_GO/UI/BP_MainHUD.PlayerInterface` (`self.HGOMainHUD`)) false))

(fn `updateInputFeedback`
  (bind _temp_inputindicator (`self.TEMP_InputIndicator`))
  (switch `ETurnState` (`self.Turn State`)
    (:`PlayerTurn`
      (`SceneComponent.SetVisibility` _temp_inputindicator (not (`self.InputBlocked`)) false))
    (:`EnemyTurn`
      (`SceneComponent.SetVisibility` _temp_inputindicator false false))))

(fn `UserConstructionScript`)