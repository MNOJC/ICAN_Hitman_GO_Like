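; String-light garland for Hitman GO that flickers when an enemy pawn stands on one of its DetectedNodeIDs.
; The construction script lays instanced lanterns and cable segments along a spline, cycling lamp colors through per-instance custom data.
; Each enemy's start node and completed moves toggle flickering, so the last one checked wins.
; A timeline drives the shared emissive material and rect light brightness, replaying after random delays.
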(event `StartFlickering`
  (if (not (`self.IsFlickering`))
    (set `self.IsFlickering` true)
    (`MaterialInstanceDynamic.SetScalarParameterValue` (`self.LampMaterialInstance`) "EmissiveIntensity" (`self.MaximumEmissiveIntensity`))
    (`LightComponent.SetIESBrightnessScale` (`self.RectLight`) (`self.MaximumLightIntensity`))
    (bind (_direction _lightflickering) (`Timeline|Timeline` :!via `PlayFromStart` :!label _label)
      (:`Update`
        (`MaterialInstanceDynamic.SetScalarParameterValue` (`self.LampMaterialInstance`) "EmissiveIntensity" (* (`self.MaximumEmissiveIntensity`) _lightflickering))
        (`LightComponent.SetIESBrightnessScale` (`self.RectLight`) (* _lightflickering (`self.MaximumLightIntensity`))))
      (:`Finished`
        (if (`self.IsFlickering`)
          (`KismetSystemLibrary.Delay` (`KismetMathLibrary.RandomFloatInRange` (`self.MinimumDelayBetweenFlickers`) (`self.MaximumDelayBetweenFlickers`)))
          (`LightComponent.SetIESBrightnessScale` (`self.RectLight`) (`self.MaximumLightIntensity`))
          (`MaterialInstanceDynamic.SetScalarParameterValue` (`self.LampMaterialInstance`) "EmissiveIntensity" (`self.MaximumEmissiveIntensity`))
          (goto _label :!via `PlayFromStart`)
          (else
            (`MaterialInstanceDynamic.SetScalarParameterValue` (`self.LampMaterialInstance`) "EmissiveIntensity" 0.0)
            (`LightComponent.SetIESBrightnessScale` (`self.RectLight`) 0.0)))))))

(event `StopFlickering`
  (`LightComponent.SetIESBrightnessScale` (`self.RectLight`) 0.0)
  (`MaterialInstanceDynamic.SetScalarParameterValue` (`self.LampMaterialInstance`) "EmissiveIntensity" 0.0)
  (set `self.IsFlickering` false)
  (goto _label :!via `Stop`))

(event `self.ReceiveBeginPlay`
  (`self.StopFlickering`)
  (`KismetSystemLibrary.Delay` 0.2)
  (bind _outactors (`GameplayStatics.GetAllActorsOfClass` "/Game/Hitman_GO/Core/BP_HGOEnemyPawn.BP_HGOEnemyPawn_C"))
  (for _array_element _outactors
    (bind _graphmovementcomponent (`HGOEnemyPawn.GraphMovementComponent` _array_element))
    (add `HGOGraphMovementComponent.OnMovementCompleted` _graphmovementcomponent (delegate `OnMovementCompleted_Event`))
    (if (`KismetArrayLibrary.Array_Contains` (`self.DetectedNodeIDs`) (`.NodeID` (break `NodeData` (`HGONodeGraphComponent.NodeData` (`HGOGraphMovementComponent.GetCurrentNode` _graphmovementcomponent)))))
      (`self.StartFlickering`)
      (else
        (`self.StopFlickering`)))))

(event `OnMovementCompleted_Event`
  (params (NewNode :type Integer))
  (if (`KismetArrayLibrary.Array_Contains` (`self.DetectedNodeIDs`) NewNode)
    (`self.StartFlickering`)
    (else
      (`self.StopFlickering`))))

(fn `UserConstructionScript`
  (bind _hism_lamp (`self.HISM_Lamp`))
  (bind _hism_lamp_2 (`self.HISM_Lamp`))
  (bind _lampcount (`self.LampCount`))
  (bind _hism_lamp_3 (`self.HISM_Lamp`))
  (bind (_randomcolor_r _randomcolor_g _randomcolor_b) (break `LinearColor` (`self.RandomColor`)))
  (bind _spline (`self.Spline`))
  (bind _hism_cable (`self.HISM_Cable`))
  (bind _returnvalue (* (* (.x (`.BoxExtent` (`KismetMathLibrary.BreakBoxSphereBounds` (`StaticMesh.GetBounds` (`self.CableMesh`))))) 2.0) (`self.CableMeshScale`)))
  (`InstancedStaticMeshComponent.ClearInstances` _hism_lamp)
  (`StaticMeshComponent.SetStaticMesh` _hism_lamp "/Game/Hitman_GO/Art/Meshes/Props/SM_lanterne.SM_lanterne")
  (bind _returnvalue_2 (`PrimitiveComponent.CreateDynamicMaterialInstance` _hism_lamp_2 1 "/Game/Hitman_GO/Materials/M_Node_Inst.M_Node_Inst" "None"))
  (`MaterialInstanceDynamic.SetVectorParameterValue` _returnvalue_2 "Color" (`self.LampBaseColor`))
  (bind _returnvalue_3 (`PrimitiveComponent.CreateDynamicMaterialInstance` _hism_lamp_2 0 "/Game/Hitman_GO/Materials/M_Lamp_Inst.M_Lamp_Inst" "None"))
  (bind _output_get (set `self.LampMaterialInstance` _returnvalue_3))
  (`MaterialInstanceDynamic.SetVectorParameterValue` _output_get "Color" (`self.LampBaseColor`))
  (for _index (range _lampcount)
    (bind _returnvalue_4 (`InstancedStaticMeshComponent.AddInstance` _hism_lamp_3 (`KismetMathLibrary.MakeTransform` (`SplineComponent.GetLocationAtDistanceAlongSpline` (`self.Spline`) (* (/ (`SplineComponent.GetSplineLength` (`self.Spline`)) (`KismetMathLibrary.Conv_IntToDouble` _lampcount)) (`KismetMathLibrary.Conv_IntToDouble` _index)) "World") (struct :`Pitch` -180.0) (`KismetMathLibrary.Conv_DoubleToVector` (`self.LampScale`))) true))
    (set `self.RandomColor` (`|GetArrayItem` (`self.LampColors`) (mod _index (`KismetArrayLibrary.Array_Length` (`self.LampColors`)))))
    (`InstancedStaticMeshComponent.SetCustomDataValue` _hism_lamp_3 _returnvalue_4 0 _randomcolor_r false)
    (`InstancedStaticMeshComponent.SetCustomDataValue` _hism_lamp_3 _returnvalue_4 1 _randomcolor_g false)
    (`InstancedStaticMeshComponent.SetCustomDataValue` _hism_lamp_3 _returnvalue_4 2 _randomcolor_b false))
  (`StaticMeshComponent.SetStaticMesh` _hism_cable (`self.CableMesh`))
  (bind _returnvalue_5 (`PrimitiveComponent.CreateDynamicMaterialInstance` _hism_cable 0 "/Game/Hitman_GO/Materials/M_Node_Inst.M_Node_Inst" "None"))
  (`MaterialInstanceDynamic.SetVectorParameterValue` _returnvalue_5 "Color" (`self.CableColor`))
  (`InstancedStaticMeshComponent.ClearInstances` (`self.HISM_Cable`))
  (for _index_2 (range (+ (`KismetMathLibrary.Round` (/ (`SplineComponent.GetSplineLength` (`self.Spline`)) _returnvalue)) 1))
    (bind _returnvalue_6 (* _returnvalue (`KismetMathLibrary.Conv_IntToDouble` _index_2)))
    (`InstancedStaticMeshComponent.AddInstance` (`self.HISM_Cable`) (`KismetMathLibrary.MakeTransform` (`SplineComponent.GetLocationAtDistanceAlongSpline` _spline _returnvalue_6 "World") (`SplineComponent.GetRotationAtDistanceAlongSpline` _spline _returnvalue_6 "World") (`KismetMathLibrary.Conv_DoubleToVector` (`self.CableMeshScale`))) true)))